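; Spawner actor that builds a train at its location on BeginPlay, using the leftover-named SpawnSemi function.
; It spawns a head, then loops twelve times, each pass adding a car and another reverse-facing head with negated MaxSpeed at a fixed tail offset.
; Mesh offsets along Y space out the pieces.
; DeleteTrigger destroys actors leaving its overlap, except BP_LaneSpawner; SpawnVehicle is never called here.
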(event `self.ReceiveBeginPlay`
  (`self.SpawnSemi`))

(event `self.DeleteTrigger.OnComponentEndOverlap`
  (params (OverlappedComponent :type "PrimitiveComponent Object Reference") (OtherActor :type "Actor Object Reference") (OtherComp :type "PrimitiveComponent Object Reference") (OtherBodyIndex :type Integer))
  (cast `/Game/Blueprints/Spawners/BP_LaneSpawner` OtherActor
    (:`CastFailed`
      (`self.K2_DestroyActor` OtherActor))))

(fn `SpawnSemi`
  (locals (Offset :type "Float (double-precision)" :default 1500.0))
  (bind (_returnvalue_roll _returnvalue_pitch _returnvalue_yaw) (`KismetMathLibrary.BreakRotator` (`self.K2_GetActorRotation`)))
  (bind _returnvalue (`self.K2_GetActorLocation`))
  (bind _returnvalue_2 (+ _returnvalue_yaw 180.0))
  (bind _returnvalue_3 (`|SpawnActorFromClass` "/Game/Blueprints/Actors/BP_TrainHead.BP_TrainHead_C" (`KismetMathLibrary.MakeTransform` _returnvalue (`KismetMathLibrary.MakeRotator` _returnvalue_roll _returnvalue_pitch _returnvalue_2)) "Undefined" "OverrideRootScale" null null))
  (`SceneComponent.K2_AddRelativeLocation` (`/Game/Blueprints/Actors/BP_TrainHead.StaticMesh` _returnvalue_3) (`KismetMathLibrary.MakeVector` 0.0 (`local.Offset`)) false false)
  (for _index (range 1 13)
    (bind _returnvalue_4 (`|SpawnActorFromClass` "/Game/Blueprints/Actors/BP_TrainCar.BP_TrainCar_C" (`KismetMathLibrary.MakeTransform` _returnvalue (`KismetMathLibrary.MakeRotator` _returnvalue_roll _returnvalue_pitch _returnvalue_2)) "Undefined" "OverrideRootScale" null null))
    (`SceneComponent.K2_AddRelativeLocation` (`/Game/Blueprints/Actors/BP_TrainCar.StaticMesh` _returnvalue_4) (`KismetMathLibrary.MakeVector` 0.0 (+ (* _index (`self.TrainLength`)) (`local.Offset`))) false false)
    (bind _returnvalue_5 (`|SpawnActorFromClass` "/Game/Blueprints/Actors/BP_TrainHead.BP_TrainHead_C" (`KismetMathLibrary.MakeTransform` _returnvalue (`KismetMathLibrary.MakeRotator` _returnvalue_roll _returnvalue_pitch _returnvalue_yaw)) "Undefined" "OverrideRootScale" null null))
    (bind _output_get (set `/Game/Blueprints/Actors/BP_TrainHead.MaxSpeed` (* -1 (stale _output_get)) _returnvalue_5))
    (`SceneComponent.K2_AddRelativeLocation` (`/Game/Blueprints/Actors/BP_TrainHead.StaticMesh` _returnvalue_5) (`KismetMathLibrary.MakeVector` 0.0 (+ (* -13 (`self.TrainLength`)) (* -1 (`local.Offset`)))) false false)))

(fn `SpawnVehicle`
  (params (VehicleClass :type "Actor Class Reference"))
  (bind (_returnvalue_roll _returnvalue_pitch _returnvalue_yaw) (`KismetMathLibrary.BreakRotator` (`self.K2_GetActorRotation`)))
  (`|SpawnActorFromClass` VehicleClass (`KismetMathLibrary.MakeTransform` (`self.K2_GetActorLocation`) (`KismetMathLibrary.MakeRotator` _returnvalue_roll _returnvalue_pitch (+ _returnvalue_yaw 180.0))) "Undefined" "OverrideRootScale" null null)
  (`SceneComponent.K2_AttachToComponent` (`self.DefaultSceneRoot`) null "None" "KeepRelative" "KeepRelative" "KeepRelative" true))

(fn `UserConstructionScript`)