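; Vehicle spawner that keeps a lane of traffic supplied in a game with a chicken character.
; BeginPlay randomly seeds either one semi or two police cars, shifting the spawn trigger and spawn point to suit.
; Any non-chicken actor entering SpawnTrigger causes another of its class to spawn at SpawnPoint, yawed 180 degrees from the spawner, sustaining that vehicle type.
; DeleteTrigger destroys actors leaving it, except lane spawners.
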(event `self.ReceiveBeginPlay`
  (if (`KismetMathLibrary.RandomBool`)
    (`self.InitSemi`)
    (else
      (`self.Init Car`))))

(event `self.SpawnTrigger.OnComponentBeginOverlap`
  (params (OverlappedComponent :type "PrimitiveComponent Object Reference") (OtherActor :type "Actor Object Reference") (OtherComp :type "PrimitiveComponent Object Reference") (OtherBodyIndex :type Integer) (bFromSweep :type Boolean) (SweepResult :type "HitResult Structure (by ref)"))
  (cast `/Game/Blueprints/Actors/BP_Chicken_Character` OtherActor
    (:`CastFailed`
      (`self.SpawnVehicle` (`GameplayStatics.GetObjectClass` OtherActor)))))

(event `self.DeleteTrigger.OnComponentEndOverlap`
  (params (OverlappedComponent :type "PrimitiveComponent Object Reference") (OtherActor :type "Actor Object Reference") (OtherComp :type "PrimitiveComponent Object Reference") (OtherBodyIndex :type Integer))
  (cast `/Game/Blueprints/Spawners/BP_LaneSpawner` OtherActor
    (:`CastFailed`
      (`self.K2_DestroyActor` OtherActor))))

(fn `Init Car`
  (bind (_returnvalue_roll _returnvalue_pitch _returnvalue_yaw) (`KismetMathLibrary.BreakRotator` (`self.K2_GetActorRotation`)))
  (bind _spawnpoint (`self.SpawnPoint`))
  (bind _spawnpoint_2 (`self.SpawnPoint`))
  (bind _returnvalue (+ _returnvalue_yaw 180.0))
  (`SceneComponent.K2_AddLocalOffset` (`self.SpawnTrigger`) (0.0 1000.0 0.0) false false)
  (`SceneComponent.K2_AddLocalOffset` _spawnpoint (0.0 700.0 0.0) false false)
  (`|SpawnActorFromClass` "/Game/Blueprints/Actors/BP_PoliceCar.BP_PoliceCar_C" (`KismetMathLibrary.MakeTransform` (`SceneComponent.K2_GetComponentLocation` _spawnpoint) (`KismetMathLibrary.MakeRotator` _returnvalue_roll _returnvalue_pitch _returnvalue) (1.0 1.0 1.0)) "Undefined" "OverrideRootScale" null null)
  (`SceneComponent.K2_AddLocalOffset` _spawnpoint_2 (0.0 -300.0 0.0) false false)
  (`|SpawnActorFromClass` "/Game/Blueprints/Actors/BP_PoliceCar.BP_PoliceCar_C" (`KismetMathLibrary.MakeTransform` (`SceneComponent.K2_GetComponentLocation` _spawnpoint_2) (`KismetMathLibrary.MakeRotator` _returnvalue_roll _returnvalue_pitch _returnvalue)) "Undefined" "OverrideRootScale" null null)
  (`SceneComponent.K2_AddLocalOffset` (`self.SpawnPoint`) (0.0 -400.0 0.0) false false))

(fn `InitSemi`
  (bind (_returnvalue_roll _returnvalue_pitch _returnvalue_yaw) (`KismetMathLibrary.BreakRotator` (`self.K2_GetActorRotation`)))
  (bind _spawnpoint (`self.SpawnPoint`))
  (`SceneComponent.K2_AddLocalOffset` (`self.SpawnTrigger`) (0.0 700.0 0.0) false false)
  (`SceneComponent.K2_AddLocalOffset` _spawnpoint (0.0 350.0 0.0) false false)
  (`|SpawnActorFromClass` "/Game/Blueprints/Actors/BP_Semi.BP_Semi_C" (`KismetMathLibrary.MakeTransform` (`SceneComponent.K2_GetComponentLocation` _spawnpoint) (`KismetMathLibrary.MakeRotator` _returnvalue_roll _returnvalue_pitch (+ _returnvalue_yaw 180.0))) "Undefined" "OverrideRootScale" null null)
  (`SceneComponent.K2_AddLocalOffset` (`self.SpawnPoint`) (0.0 -350.0 0.0) false false))

(fn `SpawnSemi`
  (bind (_returnvalue_roll _returnvalue_pitch _returnvalue_yaw) (`KismetMathLibrary.BreakRotator` (`self.K2_GetActorRotation`)))
  (`|SpawnActorFromClass` "/Game/Blueprints/Actors/BP_Semi.BP_Semi_C" (`KismetMathLibrary.MakeTransform` (`SceneComponent.K2_GetComponentLocation` (`self.SpawnPoint`)) (`KismetMathLibrary.MakeRotator` _returnvalue_roll _returnvalue_pitch (+ _returnvalue_yaw 180.0))) "Undefined" "OverrideRootScale" null null))

(fn `SpawnVehicle`
  (params (VehicleClass :type "Actor Class Reference"))
  (bind (_returnvalue_roll _returnvalue_pitch _returnvalue_yaw) (`KismetMathLibrary.BreakRotator` (`self.K2_GetActorRotation`)))
  (`|SpawnActorFromClass` VehicleClass (`KismetMathLibrary.MakeTransform` (`SceneComponent.K2_GetComponentLocation` (`self.SpawnPoint`)) (`KismetMathLibrary.MakeRotator` _returnvalue_roll _returnvalue_pitch (+ _returnvalue_yaw 180.0))) "Undefined" "OverrideRootScale" null null))

(fn `UserConstructionScript`)