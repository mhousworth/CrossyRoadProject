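; BP_TrainSignal is a railroad crossing signal with flashing lights and a bell.
; Toggle starts or stops a looping timer and the spawned bell sound, restoring the unlit mesh when off.
; The timer calls Flash, which alternates two flash meshes and their point lights through a State value.
; On overlapping a BP_LaneSpawner's lane destroyer collision, it stops the bell and destroys itself, provided the bell is not being destroyed.
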(event `self.ReceiveBeginPlay`)

(event `self.ReceiveActorBeginOverlap`
  (params (OtherActor :type "Actor Object Reference")))

(event `self.ReceiveTick`
  (params (DeltaSeconds :type "Float (single-precision)")))

(event `self.StaticMesh.OnComponentBeginOverlap`
  (params (OverlappedComponent :type "PrimitiveComponent Object Reference") (OtherActor :type "Actor Object Reference") (OtherComp :type "PrimitiveComponent Object Reference") (OtherBodyIndex :type Integer) (bFromSweep :type Boolean) (SweepResult :type "HitResult Structure (by ref)"))
  (bind _signalbell (`self.SignalBell`))
  (bind _asbp_lane_spawner (cast `/Game/Blueprints/Spawners/BP_LaneSpawner` OtherActor))
  (if (`PrimitiveComponent.IsOverlappingActor` (`/Game/Blueprints/Spawners/BP_LaneSpawner.CollisionLaneDestroyer` _asbp_lane_spawner) self)
    (if (not (`ActorComponent.IsBeingDestroyed` _signalbell))
      (`AudioComponent.Stop` _signalbell)
      (`self.K2_DestroyActor`))))

(fn `Flash`
  (bind _staticmesh (`self.StaticMesh`))
  (`/Engine/EditorBlueprintResources/StandardMacros.CompareInt` (`self.State`) 1
    (:`>`
      (`StaticMeshComponent.SetStaticMesh` _staticmesh "/Game/Models/train_signal_flash1.train_signal_flash1" :!label _label)
      (`SceneComponent.SetVisibility` (`self.PointLight2`) false false)
      (`SceneComponent.SetVisibility` (`self.PointLight1`) true false)
      (set `self.State` 1))
    (:`==`
      (`StaticMeshComponent.SetStaticMesh` _staticmesh "/Game/Models/train_signal_flash2.train_signal_flash2")
      (`SceneComponent.SetVisibility` (`self.PointLight1`) false false)
      (`SceneComponent.SetVisibility` (`self.PointLight2`) true false)
      (set `self.State` 2))
    (:`<`
      (goto _label))))

(fn `Toggle`
  (if (`self.Flashing`)
    (`KismetSystemLibrary.K2_ClearAndInvalidateTimerHandle` (`self.Timer`))
    (`StaticMeshComponent.SetStaticMesh` (`self.StaticMesh`) "/Game/Models/train_signal.train_signal")
    (`SceneComponent.SetVisibility` (`self.PointLight1`) false false)
    (`SceneComponent.SetVisibility` (`self.PointLight2`) false false)
    (set `self.Flashing` false)
    (set `self.State` 0)
    (`AudioComponent.Stop` (`self.SignalBell`))
    (else
      (bind _returnvalue (`KismetSystemLibrary.K2_SetTimer` self "Flash" 0.2 true))
      (set `self.Timer` _returnvalue)
      (set `self.Flashing` true)
      (bind _returnvalue_2 (`GameplayStatics.SpawnSoundAtLocation` "/Game/Audio/railroad-crossing_Cue.railroad-crossing_Cue" (`self.K2_GetActorLocation`) (struct) 1.0 1.0 0.0 null null))
      (set `self.SignalBell` _returnvalue_2))))

(fn `UserConstructionScript`)