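; Player-controlled chicken actor that hops in fixed grid steps in four directions, spawning and attaching a BP_Chicken as its body on BeginPlay.
; Pressing a direction key turns and squashes the chicken as a wind-up, recording the key in a KeysDown array.
; Releasing a key re-faces the chicken to the first still-held direction, or, if none remains, restores its shape and instantly offsets the root one step without sweeping.
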(event `InputAction|MoveForward`
  (params (Key :type "Key Structure"))
  (:`Pressed`
    (`self.KeyDown` 0))
  (:`Released`
    (`self.KeyUp` 0)))

(event `InputAction|MoveBack`
  (params (Key :type "Key Structure"))
  (:`Pressed`
    (`self.KeyDown` 2))
  (:`Released`
    (`self.KeyUp` 2)))

(event `InputAction|MoveRight`
  (params (Key :type "Key Structure"))
  (:`Pressed`
    (`self.KeyDown` 3))
  (:`Released`
    (`self.KeyUp` 3)))

(event `InputAction|MoveLeft`
  (params (Key :type "Key Structure"))
  (:`Pressed`
    (`self.KeyDown` 1))
  (:`Released`
    (`self.KeyUp` 1)))

(event `self.ReceiveBeginPlay`
  (bind _returnvalue (`|SpawnActorFromClass` "/Game/Blueprints/Actors/BP_Chicken.BP_Chicken_C" (`KismetMathLibrary.MakeTransform` (0.0 0.0 0.0)) "Undefined" "OverrideRootScale" null null))
  (bind _output_get (set `self.AttachedChicken` _returnvalue))
  (`SceneComponent.K2_AttachToComponent` (`Actor.RootComponent` _output_get) (`self.DefaultSceneRoot`) "None" "KeepRelative" "KeepRelative" "KeepRelative" true)
  (`SceneComponent.K2_AddRelativeLocation` (`self.DefaultSceneRoot`) (0.0 0.0 -35.0) false false))

(fn `KeyDown`
  (params (Direction :type Integer))
  (`KismetArrayLibrary.Array_Set` (`self.KeysDown`) Direction true)
  (`self.K2_SetActorRelativeTransform` (`self.AttachedChicken`) (`KismetMathLibrary.MakeTransform` (0.0 0.0 -12.0) (select `int` Direction :`0` (struct) :`1` (struct :`Yaw` 90.0) :`2` (struct :`Yaw` 180.0) :`3` (struct :`Yaw` 270.0) :!type "Rotator Structure") (1.0 1.0 0.8)) false false))

(fn `KeyUp`
  (params (Direction :type Integer))
  (locals (KeyStillDown :type Boolean))
  (`KismetArrayLibrary.Array_Set` (`self.KeysDown`) Direction)
  (set `local.KeyStillDown` false)
  (for (_array_element _array_index) (`self.KeysDown`)
    (if _array_element
      (set `local.KeyStillDown` true)
      (`self.K2_SetActorRotation` (`self.AttachedChicken`) (select `int` _array_index :`0` (struct) :`1` (struct :`Yaw` 90.0) :`2` (struct :`Yaw` 180.0) :`3` (struct :`Yaw` 270.0) :!type "Rotator Structure") false)
      (break)))
  (if (not (`local.KeyStillDown`))
    (`self.Move` Direction)))

(fn `Move`
  (params (Direction :type Integer))
  (`KismetArrayLibrary.Array_Set` (`self.KeysDown`) Direction)
  (`self.K2_SetActorRelativeTransform` (`self.AttachedChicken`) (`KismetMathLibrary.MakeTransform` (0.0 0.0 0.0) (select `int` Direction :`0` (struct) :`1` (struct :`Yaw` 90.0) :`2` (struct :`Yaw` 180.0) :`3` (struct :`Yaw` 270.0) :!type "Rotator Structure") (1.0 1.0 1.0)) false false)
  (`SceneComponent.K2_AddRelativeLocation` (`self.DefaultSceneRoot`) (select `int` Direction :`0` (110.0 0.0 0.0) :`1` (0.0 110.0 0.0) :`2` (-110.0 0.0 0.0) :`3` (0.0 -110.0 0.0) :!type "Vector Structure") false false))

(fn `UserConstructionScript`)