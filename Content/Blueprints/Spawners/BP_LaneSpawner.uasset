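; Endless lane generator for a Crossy Road-style chicken game, which builds the starting area and spawns the player.
; Weighted random picks lay grass, street, train or water lanes tile by tile with obstacles, vehicle and train spawners, then step the actor forward.
; A trigger tracking the chicken's Y adds a lane on overlap, while another destroys most actors it touches.
; A looping timer starts all trains at once.
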(event `MassTrainTrigger`
  (bind _outactors (`GameplayStatics.GetAllActorsOfClass` "/Game/Blueprints/Spawners/BP_TrainSpawner.BP_TrainSpawner_C"))
  (for _array_element _outactors
    (`/Game/Blueprints/Spawners/BP_TrainSpawner.StartTrainEvent` _array_element)))

(event `self.ReceiveBeginPlay`
  (`KismetSystemLibrary.K2_SetTimerDelegate` (delegate `MassTrainTrigger`) 8.0 true)
  (`self.InitialSpawn`)
  (`self.SpawnGrassLane` false)
  (for _ (range 5)
    (`self.SpawnGrassLane` true))
  (`self.SpawnStreetSingleLane`)
  (`self.SpawnTrainLane`)
  (`self.SpawnLane`)
  (`self.SpawnLane`))

(event `self.CollisionLaneSpawner.OnComponentBeginOverlap`
  (params (OverlappedComponent :type "PrimitiveComponent Object Reference") (OtherActor :type "Actor Object Reference") (OtherComp :type "PrimitiveComponent Object Reference") (OtherBodyIndex :type Integer) (bFromSweep :type Boolean) (SweepResult :type "HitResult Structure (by ref)"))
  (cast `/Game/Blueprints/Actors/BP_Chicken_Character` OtherActor)
  (`self.SpawnLane`))

(event `self.ReceiveTick`
  (params (DeltaSeconds :type "Float (single-precision)"))
  (bind _collisionlanespawner (`self.CollisionLaneSpawner`))
  (bind (_returnvalue_x _returnvalue_y) (`KismetMathLibrary.BreakVector` (`self.K2_GetActorLocation` (`self.ChickenCharacter`))))
  (bind (_returnvalue_x_2 _returnvalue_y_2 _returnvalue_z) (`KismetMathLibrary.BreakVector` (`SceneComponent.K2_GetComponentLocation` _collisionlanespawner)))
  (`SceneComponent.K2_SetWorldLocation` _collisionlanespawner (`KismetMathLibrary.MakeVector` _returnvalue_x_2 _returnvalue_y _returnvalue_z) false false))

(event `self.CollisionLaneDestroyer.OnComponentBeginOverlap`
  (params (OverlappedComponent :type "PrimitiveComponent Object Reference") (OtherActor :type "Actor Object Reference") (OtherComp :type "PrimitiveComponent Object Reference") (OtherBodyIndex :type Integer) (bFromSweep :type Boolean) (SweepResult :type "HitResult Structure (by ref)"))
  (cast `/Game/Blueprints/Spawners/BP_LaneSpawner` OtherActor
    (:`CastFailed`
      (cast `/Game/Blueprints/Actors/BP_TrainSignal` OtherActor
        (:`CastFailed`
          (cast `/Game/Blueprints/Actors/BP_Chicken` OtherActor
            (:`CastFailed`
              (`self.K2_DestroyActor` OtherActor))))))))

(fn `InitialSpawn`
  (bind _tileoffset (`self.TileOffset`))
  (bind _tileoffset_2 (`self.TileOffset`))
  (for _ (range 4)
    (for _index (range 23)
      (`self.SpawnObstacle` 2 (+ (`self.K2_GetActorLocation`) (`KismetMathLibrary.MakeVector` 0.0 (* _index _tileoffset_2)))))
    (`self.K2_AddActorLocalOffset` (`KismetMathLibrary.MakeVector` _tileoffset_2)))
  (for _index_2 (range 10)
    (`self.SpawnObstacle` 2 (+ (`self.K2_GetActorLocation`) (`KismetMathLibrary.MakeVector` 0.0 (* _index_2 (`self.TileOffset`))))))
  (for _index_3 (range 3)
    (bind _returnvalue (+ (`self.K2_GetActorLocation`) (`KismetMathLibrary.MakeVector` 0.0 (* (+ _index_3 10) (`self.TileOffset`)))))
    (`self.SpawnTile` 0 _returnvalue)
    (`/Engine/EditorBlueprintResources/StandardMacros.CompareInt` 1 _index_3
      (:`==`
        (bind _returnvalue_2 (`|SpawnActorFromClass` "/Game/Blueprints/Actors/BP_Chicken_Character.BP_Chicken_Character_C" (`KismetMathLibrary.MakeTransform` (+ _returnvalue (0.0 0.0 140.0))) "Undefined" "OverrideRootScale" null null))
        (bind _output_get (set `self.ChickenCharacter` _returnvalue_2))
        (bind _returnvalue_3 (`self.K2_GetActorLocation` _output_get))
        (`SceneComponent.K2_SetWorldLocation` (`self.CollisionLaneSpawner`) (+ _returnvalue_3 (-1140.0 0.0 -60.0)) false true)
        (`SceneComponent.K2_SetWorldLocation` (`self.CollisionLaneDestroyer`) (+ _returnvalue_3 (-1960.0 0.0 -120.0)) false false))))
  (for _index_4 (range 10)
    (`self.SpawnObstacle` 2 (+ (`self.K2_GetActorLocation`) (`KismetMathLibrary.MakeVector` 0.0 (* (+ _index_4 13) _tileoffset)))))
  (`self.K2_AddActorLocalOffset` (`KismetMathLibrary.MakeVector` _tileoffset)))

(fn `SpawnGrassLane`
  (params (Obstacles :type Boolean))
  (bind _tileoffset (`self.TileOffset`))
  (for _index (range 23)
    (if Obstacles
      (`/Engine/EditorBlueprintResources/StandardMacros.CompareInt` 0 (`KismetMathLibrary.RandomIntegerInRange` 0 9)
        (:`>`
          (bind _returnvalue (+ (`self.K2_GetActorLocation`) (`KismetMathLibrary.MakeVector` 0.0 (* _index _tileoffset))))
          (`self.SpawnObstacle` (`KismetMathLibrary.RandomIntegerInRange` 0 3) _returnvalue :!label _label))
        (:`==`
          (goto _label))
        (:`<`
          (`/Engine/EditorBlueprintResources/StandardMacros.CompareInt` _index 2 :!label _label_2
            (:`>`
              _)
            (:`==`
              (goto _label))
            (:`<`
              _))
          (`/Engine/EditorBlueprintResources/StandardMacros.CompareInt` _index 20
            (:`>`
              _)
            (:`==`
              (goto _label))
            (:`<`
              _))
          (`self.SpawnTile` 0 _returnvalue)))
      (else
        (goto _label_2))))
  (`self.K2_AddActorLocalOffset` (`KismetMathLibrary.MakeVector` _tileoffset)))

(fn `SpawnLane`
  (bind _returnvalue (`KismetMathLibrary.RandomInteger` 100))
  (if (< _returnvalue 40)
    (`self.SpawnGrassLane` true)
    (elif (< _returnvalue 60)
      (`self.SpawnStreetSingleLane`)
      (elif (< _returnvalue 70)
        (`self.SpawnWaterLane`)
        (else
          (`self.SpawnTrainLane`))))))

(fn `SpawnObstacle`
  (params (TileIndex :type Integer) (SpawnLocation :type "Vector Structure"))
  (bind _returnvalue (`|SpawnActorFromClass` "/Game/Blueprints/Actors/BP_Obstacle.BP_Obstacle_C" (`KismetMathLibrary.MakeTransform` SpawnLocation) "Undefined" "OverrideRootScale" null null))
  (`/Game/Blueprints/Actors/BP_Obstacle.SetTile` _returnvalue TileIndex))

(fn `SpawnStreetSingleLane`
  (bind _returnvalue (`self.K2_GetActorLocation`))
  (bind _tileoffset (`self.TileOffset`))
  (for _index (range 23)
    (`/Engine/EditorBlueprintResources/StandardMacros.CompareInt` _index 2
      (:`>`
        (`/Engine/EditorBlueprintResources/StandardMacros.CompareInt` _index 20 :!label _label
          (:`>`
            (bind _returnvalue_2 (+ _returnvalue (`KismetMathLibrary.MakeVector` 0.0 (* _index _tileoffset) -10.0)))
            (`self.SpawnTile` 1 _returnvalue_2 :!label _label_2))
          (:`==`
            (`self.SpawnObstacle` 4 _returnvalue_2 :!label _label_3))
          (:`<`
            (goto _label_2))))
      (:`==`
        (goto _label_3))
      (:`<`
        (goto _label))))
  (if (`KismetMathLibrary.RandomBool`)
    (`|SpawnActorFromClass` "/Game/Blueprints/Spawners/BP_VehicleSpawner.BP_VehicleSpawner_C" (`KismetMathLibrary.MakeTransform` _returnvalue) "Undefined" "OverrideRootScale" null null)
    (else
      (`|SpawnActorFromClass` "/Game/Blueprints/Spawners/BP_VehicleSpawner.BP_VehicleSpawner_C" (`KismetMathLibrary.MakeTransform` (+ _returnvalue (`KismetMathLibrary.MakeVector` 0.0 (* 22 _tileoffset))) (struct :`Yaw` 180.0)) "Undefined" "OverrideRootScale" null null)))
  (`self.K2_AddActorLocalOffset` (`KismetMathLibrary.MakeVector` _tileoffset)))

(fn `SpawnTile`
  (params (TileIndex :type Integer) (SpawnLocation :type "Vector Structure"))
  (bind _returnvalue (`|SpawnActorFromClass` "/Game/Blueprints/Actors/BP_Tile.BP_Tile_C" (`KismetMathLibrary.MakeTransform` SpawnLocation) "Undefined" "OverrideRootScale" null null))
  (`/Game/Blueprints/Actors/BP_Tile.SetTile` _returnvalue TileIndex))

(fn `SpawnTrainLane`
  (locals (TempTrainSignal :type "/Game/Blueprints/Actors/BP_TrainSignal Object Reference"))
  (bind _returnvalue (`self.K2_GetActorLocation`))
  (bind _tileoffset (`self.TileOffset`))
  (for _index (range 23)
    (`/Engine/EditorBlueprintResources/StandardMacros.CompareInt` _index 2
      (:`>`
        (`/Engine/EditorBlueprintResources/StandardMacros.CompareInt` _index 20 :!label _label
          (:`>`
            (bind _returnvalue_2 (+ _returnvalue (`KismetMathLibrary.MakeVector` 0.0 (* _index _tileoffset) -10.0)))
            (`self.SpawnTile` 4 _returnvalue_2 :!label _label_2)
            (`/Engine/EditorBlueprintResources/StandardMacros.CompareInt` _index 11
              (:`==`
                (bind _returnvalue_3 (`|SpawnActorFromClass` "/Game/Blueprints/Actors/BP_TrainSignal.BP_TrainSignal_C" (`KismetMathLibrary.MakeTransform` (+ _returnvalue_2 (-55.0 -55.0 0.0))) "Undefined" "OverrideRootScale" null null))
                (set `local.TempTrainSignal` _returnvalue_3))))
          (:`==`
            (`self.SpawnObstacle` 5 _returnvalue_2 :!label _label_3))
          (:`<`
            (goto _label_2))))
      (:`==`
        (goto _label_3))
      (:`<`
        (goto _label))))
  (if (`KismetMathLibrary.RandomBool`)
    (bind _returnvalue_4 (`|SpawnActorFromClass` "/Game/Blueprints/Spawners/BP_TrainSpawner.BP_TrainSpawner_C" (`KismetMathLibrary.MakeTransform` _returnvalue) "Undefined" "OverrideRootScale" null null))
    (set `/Game/Blueprints/Spawners/BP_TrainSpawner.TrainSignal` (`local.TempTrainSignal`) _returnvalue_4)
    (else
      (bind _returnvalue_5 (`|SpawnActorFromClass` "/Game/Blueprints/Spawners/BP_TrainSpawner.BP_TrainSpawner_C" (`KismetMathLibrary.MakeTransform` (+ _returnvalue (`KismetMathLibrary.MakeVector` 0.0 (* 22 _tileoffset))) (struct :`Yaw` 180.0)) "Undefined" "OverrideRootScale" null null))
      (set `/Game/Blueprints/Spawners/BP_TrainSpawner.TrainSignal` (`local.TempTrainSignal`) _returnvalue_5)))
  (`self.K2_AddActorLocalOffset` (`KismetMathLibrary.MakeVector` _tileoffset)))

(fn `SpawnWaterLane`
  (bind _tileoffset (`self.TileOffset`))
  (for _index (range 23)
    (`/Engine/EditorBlueprintResources/StandardMacros.CompareInt` _index 2
      (:`>`
        (`/Engine/EditorBlueprintResources/StandardMacros.CompareInt` _index 20 :!label _label
          (:`>`
            (bind _returnvalue (+ (`self.K2_GetActorLocation`) (`KismetMathLibrary.MakeVector` 0.0 (* _index _tileoffset) 0.0)))
            (bind _returnvalue_2 (+ _returnvalue (0.0 0.0 -20.0)))
            (`|SpawnActorFromClass` "/Game/Blueprints/Actors/BP_Water.BP_Water_C" (`KismetMathLibrary.MakeTransform` _returnvalue_2) "Undefined" "OverrideRootScale" null null :!label _label_2)
            (`/Engine/EditorBlueprintResources/StandardMacros.CompareInt` 2 (`KismetMathLibrary.RandomIntegerInRange` 0 5)
              (:`>`
                _)
              (:`==`
                _))
            (`|SpawnActorFromClass` "/Game/Blueprints/Actors/BP_Lilypad.BP_Lilypad_C" (`KismetMathLibrary.MakeTransform` _returnvalue) "Undefined" "OverrideRootScale" null null))
          (:`==`
            (`self.SpawnObstacle` 6 _returnvalue_2 :!label _label_3))
          (:`<`
            (goto _label_2))))
      (:`==`
        (goto _label_3))
      (:`<`
        (goto _label))))
  (`self.K2_AddActorLocalOffset` (`KismetMathLibrary.MakeVector` _tileoffset)))

(fn `UserConstructionScript`)